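; Deathmatch HUD Blueprint for the SW variant of Mordhau, supplying one-team scoreboard and team select widgets.
; BeginPlay runs the parent logic, then adds a collapsed scoreboard to the viewport.
; CreateTeamSelect adds a hidden team select, while Show Team Select creates a fresh visible instance each call and switches input to UI-only.
; Show SW_MOTD displays the existing SWMOTD widget.
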(event `self.ReceiveBeginPlay`
  (`parent.ReceiveBeginPlay`)
  (bind _returnvalue (`|CreateWidget` "/StarWarsMod/UI/Deathmatch/BP_OneTeamScoreboard_SW.BP_OneTeamScoreboard_SW_C" (`self.GetOwningPlayerController`) "NewEnumerator0" true false))
  (set `self.Scoreboard` _returnvalue)
  (`Widget.SetVisibility` _returnvalue "Collapsed")
  (`UserWidget.AddToViewport` _returnvalue 0))

(fn `CreateTeamSelect`
  (bind _returnvalue (`|CreateWidget` "/StarWarsMod/UI/Deathmatch/BP_OneTeamSelect_SW.BP_OneTeamSelect_SW_C" (`self.GetOwningPlayerController`)))
  (bind _output_get (set `self.TeamSelect` _returnvalue))
  (`Widget.SetVisibility` _output_get "Collapsed")
  (`UserWidget.AddToViewport` _returnvalue 0))

(fn `Show SW_MOTD`
  (`/StarWarsMod/UI/BP_SW_MOTD.Show` (`self.SW MOTD`))
  (return))

(fn `Show Team Select`
  (bind _returnvalue (`self.GetOwningPlayerController`))
  (bind _returnvalue_2 (`|CreateWidget` "/StarWarsMod/UI/Deathmatch/BP_OneTeamSelect_SW.BP_OneTeamSelect_SW_C" _returnvalue))
  (bind _output_get (set `self.TeamSelect` _returnvalue_2))
  (`Widget.SetVisibility` _output_get "Visible")
  (`UserWidget.AddToViewport` _returnvalue_2 0)
  (`WidgetBlueprintLibrary.SetInputMode_UIOnlyEx` _returnvalue _output_get))

(fn `UserConstructionScript`
  (`parent.UserConstructionScript`))