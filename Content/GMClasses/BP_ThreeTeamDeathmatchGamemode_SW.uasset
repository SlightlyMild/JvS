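; Three-team deathmatch game mode Blueprint whose only active logic fills teams with bots.
; The AddBots event spawns the requested number of Mordhau AI controllers at the world origin and requests the given team for each.
; Each bot's character profile is picked at random from the Mordhau singleton's default profiles.
; BeginPlay and Tick are disabled stubs, and no deathmatch rules are defined in these graphs.
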(event `self.AddBots`
  (params (Amount :type Integer) (Team :type Integer))
  (bind _defaultprofiles (`MordhauSingleton.DefaultProfiles` (`MordhauUtilityLibrary.GetMordhauSingleton`)))
  (if (> Amount 0)
    (for _ (range 1 (+ Amount 1))
      (bind _returnvalue (`|SpawnActorFromClass` "/Game/Mordhau/AI/BP_MordhauAIController.BP_MordhauAIController_C" (`KismetMathLibrary.MakeTransform` (0.0 0.0 0.0)) "Undefined" "OverrideRootScale" null null))
      (`self.RequestedAssignTeam` _returnvalue Team)
      (set `BotProfile.CharacterProfile` (`|GetArrayItem` _defaultprofiles (`KismetMathLibrary.RandomIntegerInRange` 0 (`KismetArrayLibrary.Array_LastIndex` _defaultprofiles))) (`MordhauAIController.BotProfile` _returnvalue)))))

(fn `UserConstructionScript`
  (`parent.UserConstructionScript`))