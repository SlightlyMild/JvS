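; Function library for a Star Wars mod of Mordhau that registers and looks up custom content in the MordhauSingleton.
; SWManageSingleton merges mod equipment, wearables, voices and faces into singleton arrays, removing only voices and male faces, which persist across map changes.
; Helpers resolve item indices, strip ranged weapons, sort hits by distance, normalize wearable colors and match the fake helmet's speed to bare head.
; Ban-all, clear and HUD test functions are empty stubs.
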(fn `ChangeFakeHelmet`
  (locals (Tier1SpeedFactor :type "Float (double-precision)") (Tier1AccelFactor :type "Float (double-precision)"))
  (bind _returnvalue (`MordhauSingleton.GetHeadWearables` (`MordhauUtilityLibrary.GetMordhauSingleton`)))
  (`/Engine/EditorBlueprintResources/StandardMacros.IsValid` (`GameplayStatics.GetGameMode` null)
    (:`Is Valid`
      (`|ExecutionSequence`
        (:`then_0`
          (set `MordhauWearable.SpeedFactor` (`MordhauWearable.SpeedFactor` (`MordhauUtilityLibrary.GetDefaultWearable` (`|ConvertAsset` (`|GetArrayItem` _returnvalue (`KismetArrayLibrary.Array_Find` _returnvalue "/Game/Mordhau/Blueprints/Wearables/Head/BP_Bare_Head.BP_Bare_Head_C"))))) (`MordhauUtilityLibrary.GetDefaultWearable` (`|ConvertAsset` (`|GetArrayItem` _returnvalue (`KismetArrayLibrary.Array_Find` _returnvalue "/StarWarsMod/zTest2cool/FakeHelmet/FakeHelmet.FakeHelmet_C"))))))))))

(fn `FormatWearableArray`
  (params (Wears :type "Array of WearableCustomization Structure"))
  (returns (FormatedWears :type "Array of WearableCustomization Structure"))
  (locals (`00Array` :type "Array of Byte") (TempArray :type "Array of WearableCustomization Structure"))
  (bind _00array (`local.00Array`))
  (bind _00array_2 (`local.00Array`))
  (bind _output_get (set `local.TempArray` Wears))
  (for (_array_element _array_index) _output_get
    (bind (_id _colors _team1colors _team2colors _pattern) (break `WearableCustomization` _array_element))
    (if (== (`KismetArrayLibrary.Array_Length` _colors) 0)
      (`KismetArrayLibrary.Array_Set` (`local.TempArray`) _array_index (make `WearableCustomization` _id _00array_2 _00array_2 _00array_2 _pattern))
      (else
        (`KismetArrayLibrary.Array_Set` (`local.TempArray`) _array_index (make `WearableCustomization` _id _colors _00array _00array _pattern)))))
  (return (`local.TempArray`)))

(fn `SWBanEquipment`
  (locals (EquipmentToBan :type "Set of MordhauEquipment Class Reference"))
  ;[1 1 1] Bans all of mordhau equipment (No longer used due to OSDK)
)

(fn `SWBanRanged`
  (locals (RangedEquipment :type "Array of Object Soft Class Reference"))
  ;[1 1 1] For maps like Yavin or SKM
  (for _ (range (+ (`KismetArrayLibrary.Array_Length` (`local.RangedEquipment`)) 1))
    (`KismetArrayLibrary.Array_RemoveItem` (`MordhauSingleton.Equipment` (`MordhauUtilityLibrary.GetMordhauSingleton`)))))

(fn `SWClear Singleton`
  (locals (NewLocalVar_9 :type "Array of UpperChestWearable Soft Class Reference") (NewLocalVar_10 :type "Array of CharacterVoice Soft Class Reference") (NewLocalVar_11 :type "Array of CharacterFace Class Reference") (NewLocalVar_12 :type "Array of LegsWearable Soft Class Reference") (NewLocalVar_13 :type "Array of HeadWearable Soft Class Reference") (NewLocalVar_14 :type "Array of MordhauEquipment Soft Class Reference")))

(fn `SWGet SWIDs`
  (returns (`Jedi LS` :type Integer) (Darthmaul :type Integer) (DarthVader :type Integer) (Dooku :type Integer) (Kyloren :type Integer) (`Luke Short LS` :type Integer) (`Light spear` :type Integer) (E11 :type Integer) (Relbyk23 :type Integer) (AnakinVoice :type Integer) (ObiwanVoice :type Integer) (`Mando helmet` :type Integer) (`Kylo Helmet` :type Integer) (`Trooper Helmet` :type Integer) (`Vador Helmet` :type Integer) (`Yoda Helmet` :type Integer) (`Anakin Head` :type Integer) (`Obiwan Head` :type Integer))
  (bind _returnvalue (`MordhauUtilityLibrary.GetMordhauSingleton`))
  (bind _returnvalue_2 (`MordhauSingleton.GetMaleVoices` _returnvalue))
  (bind _headwearables (`MordhauSingleton.HeadWearables` _returnvalue))
  (bind _malefaces (`MordhauSingleton.MaleFaces` _returnvalue))
  (bind _equipment (`MordhauSingleton.Equipment` _returnvalue))
  (return (`KismetArrayLibrary.Array_Find` _equipment "/StarWarsMod/Weapons/StandardLS/W_JediLS.W_JediLS_C") (`KismetArrayLibrary.Array_Find` _equipment "/StarWarsMod/Weapons/DarthMaul/W_DarthMaul.W_DarthMaul_C") (`KismetArrayLibrary.Array_Find` _equipment "/StarWarsMod/Weapons/DarthVader/W_DarthVader.W_DarthVader_C") (`KismetArrayLibrary.Array_Find` _equipment "/StarWarsMod/Weapons/Dooku/W_Dooku.W_Dooku_C") (`KismetArrayLibrary.Array_Find` _equipment "/StarWarsMod/Weapons/KyloRen/W_KyloRen.W_KyloRen_C") (`KismetArrayLibrary.Array_Find` _equipment "/StarWarsMod/Weapons/ShortLightsaber/W_LukeShort.W_LukeShort_C") (`KismetArrayLibrary.Array_Find` _equipment "/StarWarsMod/Weapons/Spear/W_LightSpear.W_LightSpear_C") (`KismetArrayLibrary.Array_Find` _equipment "/StarWarsMod/Weapons/Ranged/E11/W_E11.W_E11_C") (`KismetArrayLibrary.Array_Find` _equipment "/StarWarsMod/Weapons/Ranged/RelbyK23/W_RelbyK23.W_RelbyK23_C") (`KismetArrayLibrary.Array_Find` _returnvalue_2 "/SWModAssets/Audio/Voices/Anakin/AnakinVoice.AnakinVoice_C") (`KismetArrayLibrary.Array_Find` _returnvalue_2 "/SWModAssets/Audio/Voices/Obiwan/ObiwanVoice.ObiwanVoice_C") (`KismetArrayLibrary.Array_Find` _headwearables "/SWModAssets/Wearables/Helmets/Mandalorian/P_Mando_Helmet.P_Mando_Helmet_C") (`KismetArrayLibrary.Array_Find` _headwearables "/SWModAssets/Wearables/Helmets/KyloRenHelmet/P_KylorRenHelmet.P_KylorRenHelmet_C") (`KismetArrayLibrary.Array_Find` _headwearables "/SWModAssets/Wearables/Helmets/CloneTrooperPhase3/P_Trooper_HelmetPhase3.P_Trooper_HelmetPhase3_C") (`KismetArrayLibrary.Array_Find` _headwearables "/SWModAssets/Wearables/Helmets/VadorHelmet/BP_VadorHelmet.BP_VadorHelmet_C") (`KismetArrayLibrary.Array_Find` _headwearables "/SWModAssets/Wearables/Helmets/YodaHelmet/P_YodaHelmet.P_YodaHelmet_C") (`KismetArrayLibrary.Array_Find` _malefaces "/SWModAssets/Faces/Anakin/BP_AnakinHead.BP_AnakinHead_C") (`KismetArrayLibrary.Array_Find` _malefaces "/SWModAssets/Faces/ObiWan/BP_ObiWanHead.BP_ObiWanHead_C")))

(fn `SWManage Singleton`
  (params (Add :type Boolean))
  (locals (Voices :type "Array of Object Soft Class Reference") (HeadWear :type "Array of Object Soft Class Reference") (Faces :type "Array of CharacterFace Class Reference") (UpperChest :type "Array of Object Soft Class Reference") (Legs :type "Array of Object Soft Class Reference") (Equipment :type "Array of Object Soft Class Reference") (Equipment2 :type "Array of Object Soft Class Reference") (HeadWear2 :type "Array of Object Soft Class Reference") (Voices2 :type "Array of Object Soft Class Reference") (Tier1SpeedFactor :type "Float (double-precision)") (Tier1AccelFactor :type "Float (double-precision)") (HeadWear3 :type "Array of Object Soft Class Reference") (HeadWear4 :type "Array of Object Soft Class Reference") (UpperChest2 :type "Array of Object Soft Class Reference") (Legs2 :type "Array of Object Soft Class Reference") (Equipment3 :type "Array of Object Soft Class Reference") (FacesTest :type "Array of Object Class Reference") (Equipment4 :type "Array of Object Soft Class Reference") (UpperChest3 :type "Array of Object Soft Class Reference") (UpperChest4 :type "Array of Object Soft Class Reference") (Legs3 :type "Array of Object Soft Class Reference") (MeleeEquipment :type "Array of MordhauEquipment Soft Class Reference") (`UpperChest Array` :type "Array of UpperChestWearable Soft Class Reference") (HeadArray :type "Array of HeadWearable Soft Class Reference") (`Legs Array` :type "Array of LegsWearable Soft Class Reference") (`Voices Array` :type "Array of CharacterVoice Soft Class Reference") (TestSingleUpperChest :type "Object Soft Class Reference" :default "/SWModAssets/Wearables/TestFullArmor/Anakin/Torso/BP_AnakinChest.BP_AnakinChest_C") (`Voices Array_0` :type "Array of Object Soft Class Reference") (`Legs Array_0` :type "Array of Object Soft Class Reference") (HeadArray_0 :type "Array of Object Soft Class Reference") (RangedEquipment :type "Array of MordhauEquipment Soft Class Reference") (Faces_0 :type "Array of Object Class Reference") (RangedEquipment_0 :type "Array of MordhauEquipment Soft Class Reference") (SkinColors :type "MordhauColorItemTable Structure" :default (struct :`TableName` "NSLOCTEXT(\"\", \"EA72FBB34C2A1BCAA88F9DB3BE64F642\", \"Skin Caucasian\")" :`Entries` "(BlueprintGeneratedClass'\"/Game/Mordhau/Blueprints/Colors/SkinColor/BP_SkinColor1.BP_SkinColor1_C\"',BlueprintGeneratedClass'\"/Game/Mordhau/Blueprints/Colors/SkinColor/BP_SkinColor2.BP_SkinColor2_C\"',BlueprintGeneratedClass'\"/Game/Mordhau/Blueprints/Colors/SkinColor/BP_SkinColor3.BP_SkinColor3_C\"',BlueprintGeneratedClass'\"/Game/Mordhau/Blueprints/Colors/SkinColor/BP_SkinColor4.BP_SkinColor4_C\"',BlueprintGeneratedClass'\"/Game/Mordhau/Blueprints/Colors/SkinColor/BP_SkinColor5.BP_SkinColor5_C\"',BlueprintGeneratedClass'\"/Game/Mordhau/Blueprints/Colors/SkinColor/BP_SkinColor6.BP_SkinColor6_C\"',BlueprintGeneratedClass'\"/Game/Mordhau/Blueprints/Colors/SkinColor/BP_SkinColor7.BP_SkinColor7_C\"',BlueprintGeneratedClass'\"/Game/Mordhau/Blueprints/Colors/SkinColor/BP_SkinColor8.BP_SkinColor8_C\"',BlueprintGeneratedClass'\"/StarWarsMod/Blueprints/SkinColors/BP_SkinColor9.BP_SkinColor9_C\"',BlueprintGeneratedClass'\"/StarWarsMod/Blueprints/SkinColors/BP_SkinColor10.BP_SkinColor10_C\"',BlueprintGeneratedClass'\"/StarWarsMod/Blueprints/SkinColors/BP_SkinColor11.BP_SkinColor11_C\"',BlueprintGeneratedClass'\"/StarWarsMod/Blueprints/SkinColors/BP_SkinColor12.BP_SkinColor12_C\"',BlueprintGeneratedClass'\"/StarWarsMod/Blueprints/SkinColors/BP_SkinColor13.BP_SkinColor13_C\"',BlueprintGeneratedClass'\"/StarWarsMod/Blueprints/SkinColors/BP_SkinColor14.BP_SkinColor14_C\"',BlueprintGeneratedClass'\"/StarWarsMod/Blueprints/SkinColors/BP_SkinColor15.BP_SkinColor15_C\"',BlueprintGeneratedClass'\"/StarWarsMod/Blueprints/SkinColors/BP_SkinColor16.BP_SkinColor16_C\"',BlueprintGeneratedClass'\"/StarWarsMod/Blueprints/SkinColors/BP_SkinColor17.BP_SkinColor17_C\"',BlueprintGeneratedClass'\"/StarWarsMod/Blueprints/SkinColors/BP_SkinColor18.BP_SkinColor18_C\"',BlueprintGeneratedClass'\"/StarWarsMod/Blueprints/SkinColors/BP_SkinColor19.BP_SkinColor19_C\"')")) (SWModColors :type "Array of MordhauColor Class Reference") (TestColor :type "MordhauColor Class Reference" :default "BlueprintGeneratedClass'/StarWarsMod/Blueprints/SkinColors/SWTestSkin.SWTestSkin_C'") (weapon_singular_empty :type "MordhauEquipment Soft Class Reference") (head_singular_empty :type "HeadWearable Soft Class Reference") (NewLocalVar_0 :type "Array of MordhauEquipment Soft Class Reference") (NewLocalVar_1 :type "Array of HeadWearable Soft Class Reference") (NewLocalVar_2 :type "Array of LegsWearable Soft Class Reference") (NewLocalVar_3 :type "Array of MordhauEquipment Soft Class Reference") (NewLocalVar_4 :type "Array of MordhauEquipment Soft Class Reference") (NewLocalVar_5 :type "Array of CharacterVoice Soft Class Reference") (NewLocalVar_6 :type "Array of UpperChestWearable Soft Class Reference") (NewLocalVar_7 :type "Array of CharacterFace Class Reference") (NewLocalVar_8 :type "Array of CharacterFace Class Reference") (`default faces` :type "/Game/Mordhau/Blueprints/Faces/BP_MaleFace01 Soft Object Reference") (`UpperChest Array_copy` :type "Array of UpperChestWearable Soft Class Reference") (`UpperChest Array_subset` :type "Array of UpperChestWearable Soft Class Reference") (Faces_female :type "Array of CharacterFace Class Reference"))
  (bind _returnvalue (`MordhauUtilityLibrary.GetMordhauSingleton`))
  (bind _returnvalue_2 (`MordhauUtilityLibrary.GetMordhauSingleton`))
  (bind _upperchest_array_subset (`local.UpperChest Array_subset`))
  (bind _faces_female (`local.Faces_female`))
  (bind _faces (`local.Faces`))
  (bind _faces_2 (`local.Faces`))
  (bind _voices_array (`local.Voices Array`))
  (bind _headarray (`local.HeadArray`))
  (bind _voices_array_2 (`local.Voices Array`))
  (bind _legs_array (`local.Legs Array`))
  (`|ExecutionSequence`
    (:`then_0`
      (if Add
        (`|ExecutionSequence`
          (:`then_0`
            (`KismetArrayLibrary.Array_Append` (`local.MeleeEquipment`) (`local.RangedEquipment`))
            (`MordhauSingleton.SetEquipmentArray` _returnvalue_2 (`local.MeleeEquipment`)))
          (:`then_1`
            (`KismetArrayLibrary.Array_Append` _headarray (`MordhauSingleton.GetHeadWearables` _returnvalue_2))
            (`MordhauSingleton.SetHeadWearables` _returnvalue_2 _headarray))
          (:`then_2`
            (`KismetArrayLibrary.Array_Append` _legs_array (`MordhauSingleton.GetLegsWearables` _returnvalue_2))
            (`MordhauSingleton.SetLegsWearables` _returnvalue_2 _legs_array))
          (:`then_3`
            (`KismetArrayLibrary.Array_Append` _voices_array_2 (`MordhauSingleton.GetMaleVoices` _returnvalue_2))
            (`MordhauSingleton.SetMaleVoices` _returnvalue_2 _voices_array_2))
          (:`then_4`
            (`KismetArrayLibrary.Array_Append` _upperchest_array_subset (`MordhauSingleton.GetUpperChestWearables` _returnvalue_2))
            (`MordhauSingleton.SetUpperChestWearables` _returnvalue_2 _upperchest_array_subset))
          (:`then_5`
            (`KismetArrayLibrary.Array_Append` _faces_2 (`MordhauSingleton.MaleFaces` _returnvalue_2))
            (set `MordhauSingleton.MaleFaces` _faces_2 _returnvalue_2))
          (:`then_6`
            (`KismetArrayLibrary.Array_Append` _faces_female (`MordhauSingleton.FemaleFaces` _returnvalue_2))
            (set `MordhauSingleton.FemaleFaces` _faces_female _returnvalue_2)))
        (else
          ;[1 1 1] Thiese arrays are not auto reseted by mordhau on every map change so you gotta remove them manually or they'll pile up
          (for _index (range (+ (`KismetArrayLibrary.Array_Length` _voices_array) 1))
            (`KismetArrayLibrary.Array_RemoveItem` (`MordhauSingleton.GetMaleVoices` _returnvalue) (`|GetArrayItem` _voices_array _index)))
          (for _index_2 (range (+ (`KismetArrayLibrary.Array_Length` _faces) 1))
            (`KismetArrayLibrary.Array_RemoveItem` (`MordhauSingleton.MaleFaces` _returnvalue) (`|GetArrayItem` _faces _index_2))))))
    (:`then_1`)))

(fn `SWSortHitsByDistance`
  (params (Hits :type "Array of HitResult Structure"))
  (returns (`Sorted Hits` :type "Array of HitResult Structure"))
  (locals (SortedTemp :type "Array of HitResult Structure"))
  (bind _sortedtemp (`local.SortedTemp`))
  (`KismetArrayLibrary.Array_Add` (`local.SortedTemp`) (`|GetArrayItem` Hits))
  (for _array_element Hits
    (if (not (`KismetArrayLibrary.Array_Contains` (`local.SortedTemp`) _array_element))
      ;[1 1 1] faire avec larray initial
      (for (_array_element_2 _array_index) _sortedtemp
        (if (> (`.Distance` (`GameplayStatics.BreakHitResult` _array_element_2)) (`.Distance` (`GameplayStatics.BreakHitResult` _array_element)))
          (`KismetArrayLibrary.Array_Insert` _sortedtemp _array_element _array_index)
          (break)
          (elif (not (`KismetArrayLibrary.Array_IsValidIndex` _sortedtemp (+ _array_index 1)))
            (`KismetArrayLibrary.Array_Add` _sortedtemp _array_element))))))
  (return (`local.SortedTemp`)))

(fn `TestHudFunction`)