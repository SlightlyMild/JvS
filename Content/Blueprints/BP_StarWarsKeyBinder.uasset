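; Mordhau mod Blueprint that adds Star Wars custom keybinds to the main menu's keybinding settings.
; One second after BeginPlay, where cosmetic events can run, it creates a binding widget per StarWarsKeyBinds entry, using the saved primary key or the map's default if none is set.
; It registers each widget, rebuilds the scroll box to put it at the top, then applies the bindings.
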(event `self.ReceiveBeginPlay`
  (`parent.ReceiveBeginPlay`)
  (`/Engine/EditorBlueprintResources/StandardMacros.Can Execute Cosmetic Events`
    (:`True`
      (`KismetSystemLibrary.Delay` 1.0)
      (`self.Add Modifier Custom Keybinds to HUD` (`self.StarWarsKeyBinds`) (`GameplayStatics.GetPlayerController` 0)))))

(fn `Add Modifier Custom Keybinds to HUD`
  (params (CustomKeybinds :type "Map of Name to Key Structure") (PlayerController :type "PlayerController Object Reference"))
  (locals (`Custom Keybind List` :type "Array of Name") (LocalWidget :type "Array of Widget Object Reference") (CustomKeybinds :type "Map of Name to Key Structure"))
  ;[0.3125 1 0] Crazy Mike:
  ; 0. Create a function in your player controller with the following code in it, and call that function once during beginplay (i delay this until after the first frame incase hud has not been built yet)
  ;
  ; 1. Promote these two to "local" variables (make sure they are in the Local variable list and not the normal list) in this function
  ;
  ; 2. Add array members to Custom Keybind List and each member name will be your new custom input name
  ;
  ; 3. Go to your editor project settings -> inputs->action mappings and add new action mappings identical to the ones in your custom keybind list
  ;
  ; 4. In your controller / character (wherever you are calling input events from) you can now add those input events and use them similar to using a direct keyboard input
  ;
  ; 5. In the editor start playing and go to the settings -> keybinds menu and your new keybind should be visible at the top of the list and can be rebound at will and saved to the input.ini file the same as all other keybinds, and only when your mod is loaded will the input be visible and 'exist' (so it wont disrupt normal play or other mods)
  (bind _keys (`BlueprintMapLibrary.Map_Keys` CustomKeybinds))
  (bind _values (`BlueprintMapLibrary.Map_Values` (`local.CustomKeybinds`)))
  (bind _output_get (set `local.Custom Keybind List` _keys))
  (for (_array_element _array_index) _output_get
    (bind _asbp_mordhau_hud (cast `/Game/Mordhau/Blueprints/BP_MordhauHUD` (`PlayerController.GetHUD` PlayerController)))
    (bind _asbp_main_menu (cast `/Game/Mordhau/UI/Customization/BP_MainMenu` (`/Game/Mordhau/Blueprints/BP_MordhauHUD.MainMenu` _asbp_mordhau_hud)))
    (bind _returnvalue (`|CreateWidget` "/Game/Mordhau/UI/BP_KeyBindingElementWidget.BP_KeyBindingElementWidget_C" PlayerController))
    (bind _output_get_2 (set `/Game/Mordhau/UI/BP_KeyBindingElementWidget.ActionName` _array_element _returnvalue))
    (bind ((`Key` _key)) (break `InputActionKeyMapping` (`MordhauInput.GetPrimaryActionKeyBinding` (`MordhauUtilityLibrary.GetMordhauInput`) (`KismetSystemLibrary.MakeLiteralName` _array_element))))
    (bind _output (`|GetArrayItem` _values _array_index))
    (set `/Game/Mordhau/UI/BP_KeyBindingElementWidget.PrimaryBindings` (select `bool` (== _key "None") :`false` (`|MakeArray` _key _key _key _key) :`true` (`|MakeArray` _output _output _output _output)) _returnvalue)
    (bind _bp_keybindingssettings (`/Game/Mordhau/UI/Customization/BP_MainMenu.BP_KeyBindingsSettings` _asbp_main_menu))
    (`BlueprintMapLibrary.Map_Add` (`/Game/Mordhau/UI/GameSettings/BP_KeyBindingsSettings.BindingWidgets` _bp_keybindingssettings) _output_get_2 _returnvalue)
    (bind _output_get_3 (set `local.LocalWidget` (`|MakeArray` _returnvalue :!type "Widget Object Reference")))
    (bind _scrollbox_1 (`/Game/Mordhau/UI/GameSettings/BP_KeyBindingsSettings.ScrollBox_1` _bp_keybindingssettings))
    (`KismetArrayLibrary.Array_Append` _output_get_3 (`PanelWidget.GetAllChildren` _scrollbox_1))
    (`PanelWidget.ClearChildren` _scrollbox_1)
    (for _array_element_2 _output_get_3
      (`PanelWidget.AddChild` _scrollbox_1 _array_element_2)))
  (bind _asbp_mordhau_hud_2 (cast `/Game/Mordhau/Blueprints/BP_MordhauHUD` (`PlayerController.GetHUD` PlayerController)))
  (bind _asbp_main_menu_2 (cast `/Game/Mordhau/UI/Customization/BP_MainMenu` (`/Game/Mordhau/Blueprints/BP_MordhauHUD.MainMenu` _asbp_mordhau_hud_2)))
  (`/Game/Mordhau/UI/GameSettings/BP_KeyBindingsSettings.ApplyKeyBindings` (`/Game/Mordhau/UI/Customization/BP_MainMenu.BP_KeyBindingsSettings` _asbp_main_menu_2)))

(fn `UserConstructionScript`)